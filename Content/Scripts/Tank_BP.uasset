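; Tank Blueprint that keeps its actor attached to the tank body and handles orbit-style camera aiming.
; Each Tick moves the owning actor to the TankBody's world location without sweep or teleport, so the scene root follows the body.
; AimUp and AimRight axis inputs add local pitch to the SpringArm and yaw to a separate YawGimbal, keeping the two rotation axes on different components.
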(event EventBeginPlay)

(event Collision|EventActorBeginOverlap
  (params (OtherActor :type Actor%20Object%20Reference)))

(event EventTick
  (params (DeltaSeconds :type Float%20%28single-precision%29))
  ;[1 1 1] Move the scene root along with the tank body
  (Transformation|SetActorLocation (Components|GetOwner (Variables|Default|GetRootScene)) (Transformation|GetWorldLocation (Variables|Default|GetTank%20Body)) false false))

(event Input|AxisEvents|InputAxisAimRight
  (params (AxisValue :type Float%20%28single-precision%29))
  ;[1 1 1] Input to Camera Rotation
  (Transformation|AddLocalRotation (Variables|Default|GetYawGimbal) (Math|Rotator|MakeRotator 0.0 0.0 AxisValue) false false))

(event Input|AxisEvents|InputAxisAimUp
  (params (AxisValue :type Float%20%28single-precision%29))
  ;[1 1 1] Input to Camera Rotation
  (Transformation|AddLocalRotation (Variables|Default|GetSpringArm) (Math|Rotator|MakeRotator 0.0 AxisValue 0.0) false false))

(fn ConstructionScript)